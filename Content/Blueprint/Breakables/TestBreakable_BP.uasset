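; Test breakable actor that takes damage through its BreakableComponentBP when the player touches it or when it hits something while falling.
; Overlap with a ThirdPersonCharacter1 calls BreakByPlayer on the component.
; A mesh hit calls BreakByFall, crediting player pawn 0, if the mesh's downward physics velocity is at or beyond a threshold.
; Both paths print that character's Money afterwards.
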(event OnComponentHit(Mesh)
  (params (HitComponent :type Primitive%20Component%20Object%20Reference) (OtherActor :type Actor%20Object%20Reference) (OtherComp :type Primitive%20Component%20Object%20Reference) (NormalImpulse :type Vector :default "0, 0, 0") (Hit :type Hit%20Result%20Structure%20%28by%20ref%29))
  (bind _returnvalue (Physics|GetPhysicsLinearVelocity HitComponent "None"))
  (if (<= (.z _returnvalue) -2e+02)
    (bind _asthird_person_character_1 (Utilities|Casting|CastToThirdPersonCharacter1 (Game|Player|GetPlayerPawn 0)))
    (Default|BreakbyFall (Variables|Default|GetBreakableComponent_BP) 1 _asthird_person_character_1 self)
    (Development|PrintString (Utilities|String|ToString(Float) (Variables|/Game/ThirdPersonBP/Blueprints/ThirdPersonCharacter1.ThirdPersonCharacter1_C|GetMoney _asthird_person_character_1)))))

(event EventBeginPlay)

(event Collision|EventActorBeginOverlap
  (params (OtherActor :type Actor%20Object%20Reference))
  (bind _asthird_person_character_1 (Utilities|Casting|CastToThirdPersonCharacter1 OtherActor))
  (Default|BreakbyPlayer (Variables|Default|GetBreakableComponent_BP) _asthird_person_character_1 self 1)
  (Development|PrintString (Utilities|String|ToString(Float) (Variables|/Game/ThirdPersonBP/Blueprints/ThirdPersonCharacter1.ThirdPersonCharacter1_C|GetMoney _asthird_person_character_1))))

(event EventTick
  (params (DeltaSeconds :type Float%20%28single-precision%29)))

(fn ConstructionScript)