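; Breakable component that gives an object health and pays the player money equal to its Worth when it is destroyed.
; BreakByPlayer applies damage only while the player's Hitbox overlaps the target actor, whereas BreakByFall applies damage without that check.
; Once Health reaches zero or below, both events add the money, spawn an attached sparks emitter and destroy the actor.
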(event Custom|BreakByPlayer
  (params (Player :type Third%20Person%20Character%201%20Object%20Reference) (Actor :type Actor%20Object%20Reference) (Damage :type Byte))
  (Variables|Default|SetActorReference Actor)
  (if (Collision|IsOverlappingActor (Variables|/Game/ThirdPersonBP/Blueprints/ThirdPersonCharacter1.ThirdPersonCharacter1_C|GetHitbox Player) Actor :!class /Script/Engine.PrimitiveComponent)
    (Variables|Default|SetHealth (- (Variables|Default|GetHealth) Damage))
    (if (<= (Variables|Default|GetHealth) 0)
      (Variables|/Game/ThirdPersonBP/Blueprints/ThirdPersonCharacter1.ThirdPersonCharacter1_C|SetMoney Player (+ (Variables|/Game/ThirdPersonBP/Blueprints/ThirdPersonCharacter1.ThirdPersonCharacter1_C|GetMoney Player) (Variables|Default|GetWorth)))
      (Effects|SpawnEmitterAttached "/Game/StarterContent/Particles/P_Sparks.P_Sparks" 0 "None")
      (Actor|DestroyActor Actor))))

(event Custom|BreakByFall
  (params (Damage :type Byte) (Player :type Third%20Person%20Character%201%20Object%20Reference) (Actor :type Actor%20Object%20Reference))
  (Variables|Default|SetHealth (- (Variables|Default|GetHealth) Damage))
  (if (<= (Variables|Default|GetHealth) 0)
    (Variables|/Game/ThirdPersonBP/Blueprints/ThirdPersonCharacter1.ThirdPersonCharacter1_C|SetMoney Player (+ (Variables|/Game/ThirdPersonBP/Blueprints/ThirdPersonCharacter1.ThirdPersonCharacter1_C|GetMoney Player) (Variables|Default|GetWorth)))
    (Effects|SpawnEmitterAttached "/Game/StarterContent/Particles/P_Sparks.P_Sparks" 0 "None")
    (Actor|DestroyActor Actor)))

(event EventBeginPlay)

(event EventTick
  (params (DeltaSeconds :type Float%20%28single-precision%29)))